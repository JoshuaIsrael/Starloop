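; Player controller that shows the main menu on BeginPlay and hands the player a character to start the game.
; SetCharacter runs once, possessing the first BP_SLCharacter not controlled by a PlayerController and copying the PlayerState's name to it through NameComponent's ServerSetName.
; It then calls StartGame, which removes the menu, switches to game-only input and hides the cursor.
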(event `self.ReceiveBeginPlay`
  (`parent.ReceiveBeginPlay`)
  (bind _returnvalue (`|CreateWidget` "/Game/UI/Widgets/WBP_MainMenu.WBP_MainMenu_C" self))
  (`/Engine/EditorBlueprintResources/StandardMacros.IsValid` _returnvalue
    (:`Is Valid`
      (bind _output_get (set `self.Main Menu Widget` _returnvalue))
      (`UserWidget.AddToPlayerScreen` _output_get 0)
      (`WidgetBlueprintLibrary.SetInputMode_GameAndUIEx` self _output_get)
      (set `self.bShowMouseCursor` true))))

(event `Set Character`
  (`/Engine/EditorBlueprintResources/StandardMacros.DoOnce` false
    (:`Completed`
      (bind _outactors (`GameplayStatics.GetAllActorsOfClass` "/Game/Blueprints/Characters/BP_SLCharacter.BP_SLCharacter_C"))
      (for _array_element _outactors
        (cast `PlayerController` (`Pawn.GetController` _array_element)
          (:`CastFailed`
            (`self.Possess` _array_element)
            (`NameComponent.Server_SetName` (`self.GetComponentByClass` _array_element "/Script/NameModule.NameComponent") (`NameComponent.GetName` (`self.GetComponentByClass` (`self.PlayerState`) "/Script/NameModule.NameComponent")))
            (`self.Start Game`)
            (break)))))))

(event `Start Game`
  (`Widget.RemoveFromParent` (`self.Main Menu Widget`))
  (`WidgetBlueprintLibrary.SetInputMode_GameOnly` self)
  (set `self.bShowMouseCursor` false))

(fn `OnRep_Name`)

(fn `UserConstructionScript`)